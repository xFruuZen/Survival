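; Day cycle Blueprint meant to rotate a sun actor by time of day, with its update logic currently disconnected.
; BeginPlay converts a day length in minutes into seconds per day and per in-game hour.
; The unwired chain would advance the hour by delta time, map it to sun pitch and refresh the sky's sun direction.
; Tick is empty, so the sun never moves.
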(event EventBeginPlay
  (bind _output_get (Variables|Default|Seta%20Day (* (Variables|Default|GetTime%20of%20Day%20in%20Min) 6e+01)))
  (Variables|Default|Seta%20Hour (/ _output_get 24.0)))

(event EventTick
  (params (DeltaSeconds :type Float%20%28single-precision%29)))

(fn ConstructionScript)